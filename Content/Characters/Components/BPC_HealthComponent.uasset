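; BPC_HealthComponent is an actor component that tracks health and handles damage reactions for characters and barrels.
; Damage clamps CurrentHealth, fires hit, health-update and, at zero, death dispatchers, then updates the player's HUD or briefly stuns other owners by disabling movement.
; Damagflash pulses a scalar parameter on the owner's material instance, casting to BP_CharacterBase or BP_Barril to find it.
; Stun relies on the character reference cached by that flash cast.
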(event `Damagflash`
  (params (Multiplier :type "Float (double-precision)"))
  (bind _returnvalue (`self.GetOwner`))
  (bind _asbp_character_base (cast `/Game/Characters/CharacterBase/BP_CharacterBase` _returnvalue)
    (:`then`
      (bind _output_get (set `self.MITo Damage Flash` (`/Game/Characters/CharacterBase/BP_CharacterBase.MIToDamageFlash` _asbp_character_base)))
      (`MaterialInstanceDynamic.SetScalarParameterValue` _output_get "Multiplier" Multiplier)
      (`KismetSystemLibrary.Delay` 0.5)
      (`MaterialInstanceDynamic.SetScalarParameterValue` (`self.MITo Damage Flash`) "Multiplier" 0.0))
    (:`CastFailed`
      (bind _asbp_barril (cast `/Game/Blueprints/Destruibles/BP_Barril` _returnvalue))
      (bind _minstance_damage_hit (`/Game/Blueprints/Destruibles/BP_Barril.MInstance Damage Hit` _asbp_barril))
      (set `self.MInstance Damage Hit` _minstance_damage_hit)
      (`MaterialInstanceDynamic.SetScalarParameterValue` _minstance_damage_hit "MultiHit" Multiplier)
      (`KismetSystemLibrary.Delay` 0.2)
      (`MaterialInstanceDynamic.SetScalarParameterValue` (`self.MInstance Damage Hit`) "MultiHit" 0.0))))

(event `Stun`
  (if (`KismetSystemLibrary.IsValid` (stale `Damagflash` _asbp_character_base))
    (bind _charactermovement (`Character.CharacterMovement` (stale `Damagflash` _asbp_character_base)))
    (`CharacterMovementComponent.DisableMovement` _charactermovement)
    (`KismetSystemLibrary.Delay` 0.5)
    (`CharacterMovementComponent.SetMovementMode` _charactermovement "MOVE_Walking" 0)))

(fn `Damage`
  (params (Damage :type "Float (double-precision)"))
  (bind _maxhealth (`self.MaxHealth`))
  (bind _output_get (set `self.CurrentHealth` (`KismetMathLibrary.FClamp` (- (`self.CurrentHealth`) Damage) 0.0 (`self.MaxHealth`))))
  (`self.OnHit` _output_get)
  (`self.Damagflash` 1.0)
  (`self.E_HealthUpdate` _output_get _maxhealth)
  (bind _asbp_player_character (cast `/Game/Characters/Character/BP_PlayerCharacter` (`self.GetOwner`))
    (:`then`
      (`/Game/Characters/Character/UI/WBP_HUD.UpdateHealthState` (`/Game/Characters/Character/BP_PlayerCharacter.HUDReference` _asbp_player_character) _output_get _maxhealth))
    (:`CastFailed`
      (`self.Stun`)))
  (if (== _output_get 0.0)
    (`self.OnDeath`)))