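; BP_RangedEnemy is a ranged enemy that fires projectiles at the player and awards coins when killed.
; It configures its enemy type and attack slot, writes targets to the AI Blackboard, and routes RangedAttack to AtaqueDistancia.
; NotifyRangedAttack turns it toward the player on yaw and spawns BP_Proyectil_Enemy, gated by a timer cooldown.
; Health component death grants random coins, plays a sound, then destroys the actor after a short delay.
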(event `self.ReceiveBeginPlay`
  (`parent.ReceiveBeginPlay`)
  (set `self.EnemyTipe` "NewEnumerator1")
  (set `self.AtaqueADSlot` "AttackRanged")
  (add `/Game/Characters/Components/BPC_HealthComponent.OnDeath` (`self.BPC_HealthComponent`) (delegate `Death`)))

(event `Death`
  (bind _asbp_player_character (cast `/Game/Characters/Character/BP_PlayerCharacter` (`GameplayStatics.GetPlayerCharacter` 0)))
  (`/Game/Characters/Character/BP_PlayerCharacter.AddCoins` _asbp_player_character (`KismetMathLibrary.RandomIntegerInRange` 3 6))
  (`GameplayStatics.PlaySoundAtLocation` "/Game/FX/Sounds/AssetsSounds/DeathEnemy.DeathEnemy" (`self.K2_GetActorLocation`) (struct) 1.0 1.0 0.0 null null null null)
  (`KismetSystemLibrary.Delay` 0.5)
  (`self.K2_DestroyActor`))

(event `/Game/Characters/Interfaces/BPI_Enemies.SetearObjetivo`
  (params (Objetivo :type "Actor Object Reference"))
  (`BlackboardComponent.SetValueAsObject` (`AIBlueprintHelperLibrary.GetBlackboard` (`self.GetController`)) (`self.ObjetivoBBKey`) Objetivo))

(event `/Game/Characters/Interfaces/BPI_Enemies.RangedAttack`
  (`self.AtaqueDistancia`))

(event `/Game/Characters/Interfaces/BPI_Enemies.NotifyRangedAttack`
  (if (`self.Puede Disparar`)
    (`self.Disparar`)
    (set `self.Puede Disparar` false)
    (`KismetSystemLibrary.K2_SetTimer` null "HabilitarDisparo" 1.5)))

(fn `Disparar`
  (bind _asbp_player_character (cast `/Game/Characters/Character/BP_PlayerCharacter` (`GameplayStatics.GetPlayerPawn` 0))
    (:`then`
      (bind (_returnvalue_roll _returnvalue_pitch _returnvalue_yaw) (`KismetMathLibrary.BreakRotator` (`KismetMathLibrary.FindLookAtRotation` (`KismetMathLibrary.MakeVector` 0.0) (- (`self.K2_GetActorLocation` _asbp_player_character) (`self.K2_GetActorLocation`)))))
      (`self.K2_SetActorRotation` (`KismetMathLibrary.MakeRotator` 0.0 0.0 _returnvalue_yaw))
      (`|SpawnActorFromClass` "/Game/Blueprints/Proyectil/BP_Proyectil_Enemy.BP_Proyectil_Enemy_C" (`self.GetTransform`) "Undefined" "MultiplyWithRoot" null 1200.0 (`self.GetActorForwardVector`) (`self.Damage`) null))
    (:`CastFailed`
      (`KismetSystemLibrary.PrintString` "fallo el cast"))))

(fn `HabilitarDisparo`
  (set `self.Puede Disparar` true))

(fn `UserConstructionScript`)