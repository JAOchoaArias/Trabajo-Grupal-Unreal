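; Boss enemy Blueprint that sets up the inherited enemy's type and attack animations, with melee and ranged attacks and a blackboard-driven target.
; Attack events call the base attack functions, while ANBoss events apply melee damage to overlapping players or fire a player-facing projectile on a timer-reset cooldown.
; Health component death awards random coins, plays a sound, destroys the boss and opens the win menu level.
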(event `self.ReceiveBeginPlay`
  (`parent.ReceiveBeginPlay`)
  (set `self.EnemyTipe` "NewEnumerator2")
  (bind _output_get (set `self.AtaqueCaCSlot` (`self.AtaqueCaCSlot`)))
  (set `self.AtaqueADSlot` _output_get)
  (set `self.AnimacionDeAtaque` "/Game/Characters/Enemies/Animaciones/AnimSequences/AttackBoss.AttackBoss")
  (set `self.AnimacionAtaqueADistancia` "/Game/Characters/Enemies/Animaciones/AnimSequences/BossRanged.BossRanged")
  (add `/Game/Characters/Components/BPC_HealthComponent.OnDeath` (`self.BPC_HealthComponent`) (delegate `Death`)))

(event `Death`
  (bind _asbp_player_character (cast `/Game/Characters/Character/BP_PlayerCharacter` (`GameplayStatics.GetPlayerCharacter` 0)))
  (`/Game/Characters/Character/BP_PlayerCharacter.AddCoins` _asbp_player_character (`KismetMathLibrary.RandomIntegerInRange` 50 100))
  (`GameplayStatics.PlaySoundAtLocation` "/Game/FX/Sounds/AssetsSounds/DeathEnemy.DeathEnemy" (`self.K2_GetActorLocation`) (struct) 1.0 1.0 0.0 null null null null)
  (`KismetSystemLibrary.Delay` 0.5)
  (`self.K2_DestroyActor`)
  (`GameplayStatics.OpenLevel` "WinMenu"))

(event `/Game/Characters/Interfaces/BPI_Enemies.SetearObjetivo`
  (params (Objetivo :type "Actor Object Reference"))
  (`BlackboardComponent.SetValueAsObject` (`AIBlueprintHelperLibrary.GetBlackboard` (`self.GetController`)) (`self.Objetivo BBKey Padre`) Objetivo))

(event `/Game/Characters/Interfaces/BPI_Enemies.AtaqueMeleeDelJefe`
  (`self.AtaqueBase`))

(event `/Game/Characters/Interfaces/BPI_Enemies.AtaqueRangoDelJefe`
  (`self.AtaqueDistancia`))

(event `/Game/Characters/Interfaces/BPI_Enemies.ANBoss_CaC`
  (for _array_element (`PrimitiveComponent.GetOverlappingActors` (`self.Collision Attack`) "/Game/Characters/Character/BP_PlayerCharacter.BP_PlayerCharacter_C")
    (`/Game/Characters/Components/BPC_HealthComponent.Damage` (`self.GetComponentByClass` _array_element "/Game/Characters/Components/BPC_HealthComponent.BPC_HealthComponent_C") (`self.Damage`))))

(event `/Game/Characters/Interfaces/BPI_Enemies.ANBoss_AD`
  (if (`self.PuedeDisparar`)
    (`self.Disparar`)
    (set `self.PuedeDisparar` false)
    (`KismetSystemLibrary.K2_SetTimer` null "HabilitarDisparo" 1.5)))

(fn `Disparar`
  (bind _asbp_player_character (cast `/Game/Characters/Character/BP_PlayerCharacter` (`GameplayStatics.GetPlayerPawn` 0))
    (:`then`
      (bind (_returnvalue_roll _returnvalue_pitch _returnvalue_yaw) (`KismetMathLibrary.BreakRotator` (`KismetMathLibrary.FindLookAtRotation` (`KismetMathLibrary.MakeVector` 0.0) (- (`self.K2_GetActorLocation` _asbp_player_character) (`self.K2_GetActorLocation`)))))
      (`self.K2_SetActorRotation` (`KismetMathLibrary.MakeRotator` 0.0 0.0 _returnvalue_yaw))
      (`|SpawnActorFromClass` "/Game/Blueprints/Proyectil/BP_ProyectilJefe.BP_ProyectilJefe_C" (`self.GetTransform`) "Undefined" "MultiplyWithRoot" null 3000.0 (`self.GetActorForwardVector`) 100.0 null))
    (:`CastFailed`
      (`KismetSystemLibrary.PrintString` "fallo el cast"))))

(fn `HabilitarDisparo`
  (set `self.PuedeDisparar` true))

(fn `UserConstructionScript`
  (`parent.UserConstructionScript`))