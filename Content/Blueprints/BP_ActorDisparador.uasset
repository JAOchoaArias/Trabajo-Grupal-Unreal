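; BP_ActorDisparador is a trigger volume that tells a set of enemies when a player enters or leaves it.
; When an actor implementing BPI_Player begins overlapping, it passes that actor to SetearObjetivo on every entry in the Enemies array.
; When such an actor stops overlapping the Box component, it calls SetearObjetivo with no target on the same enemies.
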(event `self.ReceiveActorBeginOverlap`
  (params (OtherActor :type "Actor Object Reference"))
  (if (`KismetSystemLibrary.DoesImplementInterface` OtherActor "/Game/Character/Interfaces/BPI_Player.BPI_Player_C")
    (for _array_element (`self.Enemies`)
      (`/Game/Character/Enemies/BP_Enemigo.SetearObjetivo` _array_element OtherActor))))

(event `self.Box.OnComponentEndOverlap`
  (params (OverlappedComponent :type "PrimitiveComponent Object Reference") (OtherActor :type "Actor Object Reference") (OtherComp :type "PrimitiveComponent Object Reference") (OtherBodyIndex :type Integer))
  (if (`KismetSystemLibrary.DoesImplementInterface` OtherActor "/Game/Character/Interfaces/BPI_Player.BPI_Player_C")
    (for _array_element (`self.Enemies`)
      (`/Game/Character/Enemies/BP_Enemigo.SetearObjetivo` _array_element null))))

(fn `UserConstructionScript`)