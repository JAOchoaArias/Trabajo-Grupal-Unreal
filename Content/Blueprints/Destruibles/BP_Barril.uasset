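; BP_Barril is a destructible barrel sprite that rewards the player with coins when destroyed.
; BPCHealthComponent drives it through hit and death events, swapping to the broken sprite once health drops to a threshold.
; On death it adds a random coin amount to BP_PlayerCharacter, plays a breaking sound and destroys itself after a short delay.
; BeginPlay also stores a damage-hit dynamic material instance, which this graph does not animate.
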(event `self.ReceiveBeginPlay`
  (bind _returnvalue (`PrimitiveComponent.CreateDynamicMaterialInstance` (`self.BarrilEntero`) 0 "/Game/FX/DamageFlash/MI_DamageHit.MI_DamageHit" "None"))
  (set `self.MInstance Damage Hit` _returnvalue)
  (add `/Game/Characters/Components/BPC_HealthComponent.OnHit` (`self.BPC_HealthComponent`) (delegate `OnHit`))
  (add `/Game/Characters/Components/BPC_HealthComponent.OnDeath` (`self.BPC_HealthComponent`) (delegate `Destroy`)))

(event `OnHit`
  (params (CurrentHealthInHi :type "Float (double-precision)"))
  (if (<= CurrentHealthInHi 100.0)
    (`PaperSpriteComponent.SetSprite` (`self.BarrilEntero`) (`self.BarrilRoto`))))

(event `Destroy`
  (bind _asbp_player_character (cast `/Game/Characters/Character/BP_PlayerCharacter` (`GameplayStatics.GetPlayerCharacter` 0)))
  (`/Game/Characters/Character/BP_PlayerCharacter.AddCoins` _asbp_player_character (`KismetMathLibrary.RandomIntegerInRange` 1 5))
  (`GameplayStatics.PlaySoundAtLocation` "/Game/FX/Sounds/AssetsSounds/BarrilRompiendose.BarrilRompiendose" (`self.K2_GetActorLocation`) (struct) 1.0 1.0 0.0 null null null null)
  (`KismetSystemLibrary.Delay` 0.2)
  (`self.K2_DestroyActor`))

(fn `UserConstructionScript`)