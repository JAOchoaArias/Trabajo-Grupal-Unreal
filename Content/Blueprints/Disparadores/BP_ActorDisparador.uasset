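; BP_ActorDisparador is a trigger actor that aggros a set of enemies on the player and opens the way once they are all dead.
; On BeginPlay it binds each enemy's BPC_HealthComponent death event to a counter that destroys the Puerta door actor when the count matches the enemy total.
; Overlap by a BPI_Player actor sets it as the enemies' target through an interface message; leaving the Box clears that target.
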(event `self.ReceiveBeginPlay`
  (bind _enemies (`self.Enemies`))
  (set `self.CantidadDeEnemigos` (`KismetArrayLibrary.Array_Length` _enemies))
  (for _array_element _enemies
    (add `/Game/Characters/Components/BPC_HealthComponent.OnDeath` (`self.GetComponentByClass` _array_element "/Game/Characters/Components/BPC_HealthComponent.BPC_HealthComponent_C") (delegate `ContadorDeEnemigosMuertos`))))

(event `ContadorDeEnemigosMuertos`
  (bind _result (`/Engine/EditorBlueprintResources/StandardMacros.IncrementInt` (`self.CantidadDeMuertos`))
    (:`  `
      (if (== _result (`self.CantidadDeEnemigos`))
        (`self.K2_DestroyActor` (`self.Puerta`))))))

(event `self.ReceiveActorBeginOverlap`
  (params (OtherActor :type "Actor Object Reference"))
  (if (`KismetSystemLibrary.DoesImplementInterface` OtherActor "/Game/Characters/Interfaces/BPI_Player.BPI_Player_C")
    (for _array_element (`self.Enemies`)
      (message `/Game/Characters/Interfaces/BPI_Enemies.SetearObjetivo` _array_element OtherActor))))

(event `self.Box.OnComponentEndOverlap`
  (params (OverlappedComponent :type "PrimitiveComponent Object Reference") (OtherActor :type "Actor Object Reference") (OtherComp :type "PrimitiveComponent Object Reference") (OtherBodyIndex :type Integer))
  (if (`KismetSystemLibrary.DoesImplementInterface` OtherActor "/Game/Characters/Interfaces/BPI_Player.BPI_Player_C")
    (message `/Game/Characters/Interfaces/BPI_Enemies.SetearObjetivo` (`self.Enemies`) null)))

(fn `UserConstructionScript`)