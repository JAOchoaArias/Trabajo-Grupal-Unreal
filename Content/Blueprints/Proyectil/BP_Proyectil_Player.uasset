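; BP_Proyectil_Player is a projectile, named as the player's, that damages actors it overlaps.
; On BeginPlay it sets the ProjectileMovement initial and max speed from Speed, aims its velocity along Direccion, and destroys itself after a short fixed delay.
; An overlap with any actor that has a BPC_HealthComponent applies Damage through that component and destroys the projectile; actors without one are ignored.
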(event `self.ReceiveActorBeginOverlap`
  (params (OtherActor :type "Actor Object Reference"))
  (bind _returnvalue (`self.GetComponentByClass` OtherActor "/Game/Characters/Components/BPC_HealthComponent.BPC_HealthComponent_C"))
  (`/Engine/EditorBlueprintResources/StandardMacros.IsValid` _returnvalue
    (:`Is Valid`
      (`/Game/Characters/Components/BPC_HealthComponent.Damage` _returnvalue (`self.Damage`))
      (`self.K2_DestroyActor`))))

(event `self.ReceiveBeginPlay`
  (bind _projectilemovement (`self.ProjectileMovement`))
  (bind _output_get (set `ProjectileMovementComponent.InitialSpeed` (`self.Speed`) _projectilemovement))
  (bind _output_get_2 (set `ProjectileMovementComponent.MaxSpeed` _output_get _projectilemovement))
  (set `MovementComponent.Velocity` (* _output_get_2 (`self.Direccion`)) _projectilemovement)
  (`KismetSystemLibrary.Delay` 0.5)
  (`self.K2_DestroyActor`))

(fn `UserConstructionScript`)