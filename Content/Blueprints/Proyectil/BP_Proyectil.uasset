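; BP_Proyectil is a short-lived projectile actor that damages BP_Dummy actors on overlap.
; On BeginPlay it configures its ProjectileMovement from the Speed and Direccion variables, then destroys itself after a brief delay.
; Overlapping a BP_Dummy applies fixed damage through that dummy's BPCHealthComponent and destroys the projectile, while other actors are ignored.
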(event `self.ReceiveActorBeginOverlap`
  (params (OtherActor :type "Actor Object Reference"))
  (bind _asbp_dummy (cast `/Game/Character/Enemies/BP_Dummy` OtherActor))
  (`/Game/Character/Components/BPC_HealthComponent.Damage` (`/Game/Character/Enemies/BP_Dummy.BPC_HealthComponent` _asbp_dummy) 50.0)
  (`self.K2_DestroyActor`))

(event `self.ReceiveBeginPlay`
  (bind _projectilemovement (`self.ProjectileMovement`))
  (bind _output_get (set `ProjectileMovementComponent.InitialSpeed` (`self.Speed`) _projectilemovement))
  (bind _output_get_2 (set `ProjectileMovementComponent.MaxSpeed` _output_get _projectilemovement))
  (set `MovementComponent.Velocity` (* _output_get_2 (`self.Direccion`)) _projectilemovement)
  (`KismetSystemLibrary.Delay` 0.5)
  (`self.K2_DestroyActor`))

(fn `UserConstructionScript`)