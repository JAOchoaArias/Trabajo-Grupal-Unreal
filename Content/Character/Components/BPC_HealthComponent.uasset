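; Health component for characters that tracks current health and applies incoming damage through its Damage function.
; Damage subtracts from current health clamped between zero and the maximum, fires the EHealthUpdate dispatcher and updates the HUD progress bar directly through a stored reference.
; Death at zero health only prints a Spanish debug message; otherwise the remaining health is printed on screen.
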(fn `Damage`
  (params (Damage :type "Float (double-precision)"))
  (bind _maxhealth (`self.MaxHealth`))
  (bind _output_get (set `self.CurrentHealth` (`KismetMathLibrary.FClamp` (- (`self.CurrentHealth`) Damage) 0.0 (`self.MaxHealth`))))
  (`self.E_HealthUpdate` _output_get _maxhealth)
  (`/Game/Character/Character/WBP_HUD.SetProgressBar` (`self.HUDReference`) _output_get _maxhealth)
  (if (== _output_get 0.0)
    (`KismetSystemLibrary.PrintString` "El personaje murio" true true (struct :`R` 1.0 :`B` 0.360246 :`A` 1.0) 60.0)
    (else
      (`KismetSystemLibrary.PrintString` (`KismetStringLibrary.Conv_DoubleToString` _output_get) true true (struct :`R` 0.972319 :`B` 1.0 :`A` 1.0) 60.0))))