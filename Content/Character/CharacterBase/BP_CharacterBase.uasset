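; Base character Blueprint that provides melee and ranged attack events, using PaperZD-style animation overrides.
; AtaqueBase launches the character along its forward vector and plays the melee animation at increased speed, while AtaqueDistancia plays the ranged animation in its own slot.
; Both share the Atacando flag, set when playback starts and cleared on completion, to block overlapping attacks.
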(event `AtaqueBase`
  (if (not (`self.Atacando`))
    (`self.LaunchCharacter` (* (`self.GetActorForwardVector`) (`self.ImpusloDeAtaque`)) true)
    (`PaperZDPlaySlotOverrideAction.PlayAnimationOverrideWithCallbacks` (`PaperZDAnimationComponent.AnimInstance` (`self.AnimationComponent`)) (`self.AnimacionDeAtaque`) (`self.AtaqueCaCSlot`) 1.5
      (:`then`
        (set `self.Atacando` true))
      (:`OnCompleted`
        (set `self.Atacando` false)))))

(event `AtaqueDistancia`
  (if (not (`self.Atacando`))
    (`PaperZDPlaySlotOverrideAction.PlayAnimationOverrideWithCallbacks` (`PaperZDAnimationComponent.AnimInstance` (`self.AnimationComponent`)) (`self.AnimacionAtaqueADistancia`) "AttackRanged"
      (:`then`
        (set `self.Atacando` true))
      (:`OnCompleted`
        (set `self.Atacando` false)))))

(fn `UserConstructionScript`)