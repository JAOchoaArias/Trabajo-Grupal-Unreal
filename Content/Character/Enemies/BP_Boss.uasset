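; Boss enemy Blueprint, built on a shared enemy parent, with melee and ranged attacks and a delayed destroy on health-component death.
; It writes its target to the AI Blackboard and forwards attack requests to base and ranged attack functions.
; ANBoss events apply the hits: melee damages players overlapping CollisionAttack.
; Ranged turns the boss toward player 0 and spawns a forward projectile, throttled by a timer-reset cooldown flag.
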(event `self.ReceiveBeginPlay`
  (set `self.EnemyTipe` "NewEnumerator2")
  (set `self.AtaqueADSlot` "BossAttack")
  (set `self.AtaqueADSlot` "BossAttack")
  (add `/Game/Character/Components/BPC_HealthComponent.OnDeath` (`self.BPC_HealthComponent`) (delegate `Death`)))

(event `Death`
  (`KismetSystemLibrary.Delay` 0.5)
  (`self.K2_DestroyActor`))

(event `/Game/Character/Interfaces/BPI_Enemies.SetearObjetivo`
  (params (Objetivo :type "Actor Object Reference"))
  (`BlackboardComponent.SetValueAsObject` (`AIBlueprintHelperLibrary.GetBlackboard` (`self.GetController`)) (`self.Objetivo BBKey Padre`) Objetivo))

(event `/Game/Character/Interfaces/BPI_Enemies.AtaqueEnemigo`
  (`self.AtaqueBase`))

(event `/Game/Character/Interfaces/BPI_Enemies.RangedAttack`
  (`self.AtaqueDistancia`))

(event `/Game/Character/Interfaces/BPI_Enemies.ANBoss_CaC`
  (for _array_element (`PrimitiveComponent.GetOverlappingActors` (`self.Collision Attack`) "/Game/Character/Character/BP_PlayerCharacter.BP_PlayerCharacter_C")
    (`/Game/Character/Components/BPC_HealthComponent.Damage` (`self.GetComponentByClass` _array_element "/Game/Character/Components/BPC_HealthComponent.BPC_HealthComponent_C") (`self.Damage`))))

(event `/Game/Character/Interfaces/BPI_Enemies.ANBoss_AD`
  (if (`self.PuedeDisparar`)
    (`self.Disparar`)
    (set `self.PuedeDisparar` false)
    (`KismetSystemLibrary.K2_SetTimer` null "HabilitarDisparo" 1.5)))

(fn `Disparar`
  (bind _asbp_player_character (cast `/Game/Character/Character/BP_PlayerCharacter` (`GameplayStatics.GetPlayerPawn` 0))
    (:`then`
      (bind (_returnvalue_roll _returnvalue_pitch _returnvalue_yaw) (`KismetMathLibrary.BreakRotator` (`KismetMathLibrary.FindLookAtRotation` (`KismetMathLibrary.MakeVector` 0.0) (- (`self.K2_GetActorLocation` _asbp_player_character) (`self.K2_GetActorLocation`)))))
      (`self.K2_SetActorRotation` (`KismetMathLibrary.MakeRotator` 0.0 0.0 _returnvalue_yaw))
      (`|SpawnActorFromClass` "/Game/Blueprints/Proyectil/BP_Proyectil_Enemy.BP_Proyectil_Enemy_C" (`self.GetTransform`) "Undefined" "MultiplyWithRoot" null 3000.0 (`self.GetActorForwardVector`) 15.0 null))
    (:`CastFailed`
      (`KismetSystemLibrary.PrintString` "fallo el cast"))))

(fn `HabilitarDisparo`
  (set `self.PuedeDisparar` true))

(fn `UserConstructionScript`
  (`parent.UserConstructionScript`))