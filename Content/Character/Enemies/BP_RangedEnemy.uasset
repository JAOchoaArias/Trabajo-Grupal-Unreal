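; BP_RangedEnemy is a ranged enemy character that fires BP_Proyectil_Enemy projectiles.
; It sets its enemy type on begin play, writes its target to a Blackboard key through SetearObjetivo, and triggers attacks through RangedAttack.
; NotifyRangedAttack calls Disparar, then blocks firing until a timer calls HabilitarDisparo.
; Disparar offsets the spawn location one unit toward player 0, independent of the Blackboard target, and passes no rotation.
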(event `self.ReceiveBeginPlay`
  (set `self.EnemyTipe` "NewEnumerator1"))

(event `/Game/Character/Interfaces/BPI_Enemies.SetearObjetivo`
  (params (Objetivo :type "Actor Object Reference"))
  (`BlackboardComponent.SetValueAsObject` (`AIBlueprintHelperLibrary.GetBlackboard` (`self.GetController`)) (`self.ObjetivoBBKey`) Objetivo))

(event `/Game/Character/Interfaces/BPI_Enemies.RangedAttack`
  (`self.RangedAttack`))

(event `/Game/Character/Interfaces/BPI_Enemies.NotifyRangedAttack`
  (if (`self.Puede Disparar`)
    (`self.Disparar`)
    (set `self.Puede Disparar` false)
    (`KismetSystemLibrary.K2_SetTimer` null "HabilitarDisparo" 1.5)))

(fn `Disparar`
  (`|SpawnActorFromClass` "/Game/Blueprints/Proyectil/BP_Proyectil_Enemy.BP_Proyectil_Enemy_C" (`KismetMathLibrary.Conv_VectorToTransform` (+ (`self.K2_GetActorLocation`) (`KismetMathLibrary.GetForwardVector` (`KismetMathLibrary.MakeRotFromX` (`KismetMathLibrary.Normal` (- (`self.K2_GetActorLocation` (`GameplayStatics.GetPlayerCharacter` 0)) (`self.K2_GetActorLocation`))))))) "Undefined" "MultiplyWithRoot" null null))

(fn `HabilitarDisparo`
  (set `self.Puede Disparar` true))

(fn `UserConstructionScript`)