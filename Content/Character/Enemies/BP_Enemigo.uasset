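; Enemy character Blueprint that receives a target, attacks the player and is destroyed shortly after its health component reports death.
; SetearObjetivo writes the target to the AI controller's Blackboard, and AtaqueEnemigo triggers the attack logic inherited from the parent's AtaqueBase.
; NotificacionAtaque applies damage through the health component of each player character overlapping the attack collision.
; Debug spheres for three radii remain in the graph but never run.
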(event `self.ReceiveBeginPlay`
  (`parent.ReceiveBeginPlay`)
  (set `self.EnemyTipe_0` "NewEnumerator0")
  (add `/Game/Character/Components/BPC_HealthComponent.OnDeath` (`self.BPC_HealthComponent1`) (delegate `Death Actor`)))

(event `Death Actor`
  (`KismetSystemLibrary.Delay` 0.5)
  (`self.K2_DestroyActor`))

(event `self.ReceiveTick`
  (params (DeltaSeconds :type "Float (single-precision)")))

(event `/Game/Character/Interfaces/BPI_Enemies.SetearObjetivo`
  (params (Objetivo :type "Actor Object Reference"))
  (`BlackboardComponent.SetValueAsObject` (`AIBlueprintHelperLibrary.GetBlackboard` (`self.GetController`)) (`self.ObjetivoBBKeyName`) Objetivo))

(event `/Game/Character/Interfaces/BPI_Enemies.AtaqueEnemigo`
  (`self.AtaqueBase`))

(event `/Game/Character/Interfaces/BPI_Enemies.NotificacionAtaque`
  (for _array_element (`PrimitiveComponent.GetOverlappingActors` (`self.Collision Attack`) "/Game/Character/Character/BP_PlayerCharacter.BP_PlayerCharacter_C")
    (`/Game/Character/Components/BPC_HealthComponent.Damage` (`self.GetComponentByClass` _array_element "/Game/Character/Components/BPC_HealthComponent.BPC_HealthComponent_C") (`self.Damage`))))

(fn `AtaqueBase`
  (`parent.AtaqueBase`))

(fn `UserConstructionScript`
  (`parent.UserConstructionScript`))