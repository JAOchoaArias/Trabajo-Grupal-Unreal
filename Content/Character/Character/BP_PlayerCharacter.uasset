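; Player character with switchable melee and ranged combat, world-axis Enhanced Input movement, a HUD linked to its health component and a pause menu toggle.
; Melee plays a PaperZD animation override that blocks movement, with NotifyAttack damaging BP_Dummy actors overlapping the attack collision.
; Ranged mode shows the cursor, turns the character toward the point under it and spawns BP_Proyectil, rate-limited by a timer.
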(event `self.ReceiveBeginPlay`
  (`parent.ReceiveBeginPlay`)
  ;[1 1 1] Controlar el personaje
  (bind _asplayer_controller (cast `PlayerController` (`self.GetController`)))
  (`EnhancedInputSubsystemInterface.AddMappingContext` (pcsubsystem `EnhancedInputLocalPlayerSubsystem` _asplayer_controller) "/Game/Inputs/IMC_Default.IMC_Default" 0 (struct))
  ;[1 1 1] HUD
  (bind _returnvalue (`|CreateWidget` "/Game/Character/Character/UI/WBP_HUD.WBP_HUD_C"))
  (`UserWidget.AddToViewport` _returnvalue 0)
  (set `/Game/Character/Components/BPC_HealthComponent.HUDReference` _returnvalue (`self.BPC_HealthComponent`)))

(event `EnhancedInput|/Game/Inputs/InputActions/IA_Movimiento`
  (params (ActionValue :type "Vector2D Structure") (ElapsedSeconds :type "Float (double-precision)") (TriggeredSeconds :type "Float (double-precision)") (InputAction :type "InputAction Object Reference" :default "/Game/Inputs/InputActions/IA_Movimiento.IA_Movimiento"))
  ;[1 1 1] Movimiento
  (:`Triggered`
    (if (not (`self.bAttack`))
      (`self.AddMovementInput` (1.0 0.0 0.0) ActionValue_X)
      (`self.AddMovementInput` (0.0 1.0 0.0) ActionValue_Y))))

(event `EnhancedInput|/Game/Inputs/InputActions/IA_PausedGame`
  (params (ActionValue :type Boolean) (ElapsedSeconds :type "Float (double-precision)") (TriggeredSeconds :type "Float (double-precision)") (InputAction :type "InputAction Object Reference" :default "/Game/Inputs/InputActions/IA_PausedGame.IA_PausedGame"))
  (bind _returnvalue (`GameplayStatics.GetPlayerController` 0))
  ;[1 1 1] Menu de pausa
  (:`Started`
    (if (not (`self.PausedMenuOpen`))
      (set `self.PausedMenuOpen` true)
      (bind _returnvalue_2 (`|CreateWidget` "/Game/UI/WB_PauseMenu.WB_PauseMenu_C" _returnvalue))
      (bind _output_get (set `self.Paused Menu Widget` _returnvalue_2))
      (`UserWidget.AddToViewport` _output_get 0)
      (`WidgetBlueprintLibrary.SetInputMode_GameAndUIEx` _returnvalue (`self.Paused Menu Widget`))
      (set `PlayerController.bShowMouseCursor` true (`GameplayStatics.GetPlayerController` 0))
      (`GameplayStatics.SetGamePaused` true)
      (else
        (set `self.PausedMenuOpen` false)
        (`Widget.RemoveFromParent` (`self.Paused Menu Widget`))
        (`GameplayStatics.SetGamePaused` false)
        (`WidgetBlueprintLibrary.SetInputMode_GameOnly` _returnvalue)
        (set `PlayerController.bShowMouseCursor` false (`GameplayStatics.GetPlayerController` 0))))))

(event `EnhancedInput|/Game/Inputs/InputActions/IA_StateMelee`
  (params (ActionValue :type Boolean) (ElapsedSeconds :type "Float (double-precision)") (TriggeredSeconds :type "Float (double-precision)") (InputAction :type "InputAction Object Reference" :default "/Game/Inputs/InputActions/IA_StateMelee.IA_StateMelee"))
  ;[1 1 1] Estados
  (:`Started`
    (set `self.State` "NewEnumerator0")
    (set `PlayerController.bShowMouseCursor` false (`GameplayStatics.GetPlayerController` 0))))

(event `EnhancedInput|/Game/Inputs/InputActions/IA_Attack1`
  (params (ActionValue :type Boolean) (ElapsedSeconds :type "Float (double-precision)") (TriggeredSeconds :type "Float (double-precision)") (InputAction :type "InputAction Object Reference" :default "/Game/Inputs/InputActions/IA_Attack1.IA_Attack1"))
  ;[1 1 1] Ataque
  (:`Started`
    (switch `/Game/Character/E_State` (`self.State`)
      (:`NewEnumerator0`
        (if (not (`self.bAttack`))
          (`PaperZDPlaySlotOverrideAction.PlayAnimationOverrideWithCallbacks` (`PaperZDAnimationComponent.AnimInstance` (`self.AnimationComponent`)) "/Game/Character/Animations/AnimSequences/Attack1.Attack1" "Attack1" 2.0
            (:`then`
              (set `self.bAttack` true))
            (:`OnCompleted`
              (set `self.bAttack` false :!label _label))
            (:`OnCancelled`
              (goto _label)))))
      (:`NewEnumerator1`
        (if (`self.PuedeDisparar`)
          (`self.Disparar`)
          (set `self.PuedeDisparar` false)
          (`KismetSystemLibrary.K2_SetTimer` null "HabilitarDisparo" 0.9))))))

(event `EnhancedInput|/Game/Inputs/InputActions/IA_StateRange`
  (params (ActionValue :type Boolean) (ElapsedSeconds :type "Float (double-precision)") (TriggeredSeconds :type "Float (double-precision)") (InputAction :type "InputAction Object Reference" :default "/Game/Inputs/InputActions/IA_StateRange.IA_StateRange"))
  ;[1 1 1] Estados
  (:`Started`
    (set `self.State` "NewEnumerator1")
    (set `PlayerController.bShowMouseCursor` true (`GameplayStatics.GetPlayerController` 0))))

(event `/Game/Character/CharacterBase/BPI_AttackNotify.NotifyAttack`
  ;[1 1 1] Comprobar si golpea
  (for _array_element (`PrimitiveComponent.GetOverlappingActors` (`self.Collision Attack`) "/Game/Character/Enemies/BP_Dummy.BP_Dummy_C")
    (`/Game/Character/Components/BPC_HealthComponent.Damage` (`self.GetComponentByClass` _array_element "/Game/Character/Components/BPC_HealthComponent.BPC_HealthComponent_C") (`self.DmgCharacter`))))

(fn `Disparar`
  (bind (_returnvalue_roll _returnvalue_pitch _returnvalue_yaw) (`KismetMathLibrary.BreakRotator` (`KismetMathLibrary.FindLookAtRotation` (`KismetMathLibrary.MakeVector` 0.0) (- (`.ImpactPoint` (`GameplayStatics.BreakHitResult` (`PlayerController.GetHitResultUnderCursorByChannel` (`GameplayStatics.GetPlayerController` 0) "TraceTypeQuery1" true))) (`self.K2_GetActorLocation`)))))
  (`self.K2_SetActorRotation` (`KismetMathLibrary.MakeRotator` 0.0 0.0 _returnvalue_yaw))
  (`|SpawnActorFromClass` "/Game/Blueprints/Proyectil/BP_Proyectil.BP_Proyectil_C" (`self.GetTransform`) "Undefined" "MultiplyWithRoot" null 3000.0 (`self.GetActorForwardVector`) null))

(fn `HabilitarDisparo`
  (set `self.PuedeDisparar` true))

(fn `UserConstructionScript`
  (`parent.UserConstructionScript`))